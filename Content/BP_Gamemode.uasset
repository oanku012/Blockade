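; BP_Gamemode is the game mode that handles the end of a level, showing either a level complete or game over screen.
; GoalReached shows W_LevelComplete with UI-only input and sets a Won flag.
; YouDied waits briefly so a win takes priority, then, if not won, shows W_GameOver with the AP-or-damage reason, switches to UI-only input and hides the player's cube.
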(event Custom|GoalReached
  (bind _asbp_game_state (Utilities|Casting|CastToBP_GameState (Game|GetGameState)))
  (bind _returnvalue (UserInterface|CreateWidget "/Game/W_LevelComplete.W_LevelComplete_C"))
  (UserInterface|Viewport|AddtoViewport _returnvalue 0)
  (Input|SetInputModeUIOnly (Game|GetPlayerController 0) _returnvalue "DoNotLock")
  (Variables|Default|SetWon true))

(event Custom|You%20Died
  (params (apOrDamage :type Boolean))
  (Utilities|FlowControl|Delay 0.1)
  (if (not (Variables|Default|GetWon))
    (bind _returnvalue (UserInterface|CreateWidget "/Game/W_GameOver.W_GameOver_C"))
    (Default|SetGameOverReason _returnvalue apOrDamage)
    (UserInterface|Viewport|AddtoViewport _returnvalue 0)
    (Input|SetInputModeUIOnly (Game|GetPlayerController 0) _returnvalue "DoNotLock")
    (bind _asbp_player_character (Utilities|Casting|CastToBP_PlayerCharacter (Game|Player|GetPlayerPawn 0)))
    (Development|SetHiddeninGame (Variables|/Game/BP_PlayerCharacter.BP_PlayerCharacter_C|GetCube _asbp_player_character) true true)))

(fn ConstructionScript)