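; BP_MapTile is a map tile actor that finds and stores references to its four neighboring tiles.
; On BeginPlay, it fires short Visibility line traces from its location along the positive and negative world X and Y axes, with persistent debug drawing.
; Each blocking hit that casts to BP_MapTile fills the matching Forward, Back, Right or Left tile variable, linking tiles by placement alone.
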(event EventBeginPlay
  (bind _returnvalue (Transformation|GetActorTransform))
  (Utilities|FlowControl|Sequence
    (:then_0
      (bind _outhit (Collision|LineTraceByChannel (.location _returnvalue) (+ (.location _returnvalue) "150.000000,0,0") "TraceTypeQuery1" false 0 "Persistent"))
      (if (.bBlockingHit (Collision|BreakHitResult _outhit))
        (bind _asbp_map_tile (Utilities|Casting|CastToBP_MapTile (.HitActor (Collision|BreakHitResult _outhit))))
        (Variables|Default|SetForwardTile _asbp_map_tile)))
    (:then_1
      (bind _outhit_2 (Collision|LineTraceByChannel (.location _returnvalue) (+ (.location _returnvalue) "-150.000000,0,0") "TraceTypeQuery1" false 0 "Persistent"))
      (if (.bBlockingHit (Collision|BreakHitResult _outhit_2))
        (bind _asbp_map_tile_2 (Utilities|Casting|CastToBP_MapTile (.HitActor (Collision|BreakHitResult _outhit_2))))
        (Variables|Default|SetBackTile _asbp_map_tile_2)))
    (:then_2
      (bind _outhit_3 (Collision|LineTraceByChannel (.location _returnvalue) (+ (.location _returnvalue) "0.000000,150.000000,0") "TraceTypeQuery1" false 0 "Persistent"))
      (if (.bBlockingHit (Collision|BreakHitResult _outhit_3))
        (bind _asbp_map_tile_3 (Utilities|Casting|CastToBP_MapTile (.HitActor (Collision|BreakHitResult _outhit_3))))
        (Variables|Default|SetRightTile _asbp_map_tile_3)))
    (:then_3
      (bind _outhit_4 (Collision|LineTraceByChannel (.location _returnvalue) (+ (.location _returnvalue) "0.000000,-150.000000,0") "TraceTypeQuery1" false 0 "Persistent"))
      (if (.bBlockingHit (Collision|BreakHitResult _outhit_4))
        (bind _asbp_map_tile_4 (Utilities|Casting|CastToBP_MapTile (.HitActor (Collision|BreakHitResult _outhit_4))))
        (Variables|Default|SetLeftTile _asbp_map_tile_4)))))

(event Collision|EventActorBeginOverlap
  (params (OtherActor :type Actor%20Object%20Reference)))

(event EventTick
  (params (DeltaSeconds :type Float%20%28single-precision%29)))

(fn ConstructionScript)