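; BP_MapTile is a grid map tile actor that links to its traversable neighbors and can be highlighted.
; On BeginPlay, a traversable tile line-traces along ±X and ±Y to store adjacent traversable tiles, which GetConnectedTiles returns.
; The construction script creates a dynamic material instance whose border color and intensity drive highlighting.
; Highlight and StopHighlight act only on highlightable tiles, while SetTileColor changes the border color unconditionally.
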(event Custom|SetTileColor
  (params (Value :type Linear%20Color%20Structure))
  (Rendering|Material|SetVectorParameterValue (Variables|Default|GetMaterialInstance) "BorderColor" Value :!class /Script/Engine.MaterialInstanceDynamic))

(event Custom|TestColor
  (CallFunction|SetTileCOlor "(R=0.000000,G=1.000000,B=0.385502,A=1.000000)"))

(event Custom|Highlight
  (params (Value :type Linear%20Color%20Structure))
  (bind _materialinstance (Variables|Default|GetMaterialInstance))
  (if (Variables|Default|GetIsHighlightable)
    (Rendering|Material|SetVectorParameterValue _materialinstance "BorderColor" Value :!class /Script/Engine.MaterialInstanceDynamic)
    (Rendering|Material|SetScalarParameterValue _materialinstance "Intensity" 1.0 :!class /Script/Engine.MaterialInstanceDynamic)))

(event Custom|StopHighlight
  (bind _materialinstance (Variables|Default|GetMaterialInstance))
  (if (Variables|Default|GetIsHighlightable)
    (Rendering|Material|SetVectorParameterValue _materialinstance "BorderColor" (Variables|Default|GetDefaultColor) :!class /Script/Engine.MaterialInstanceDynamic)
    (Rendering|Material|SetScalarParameterValue _materialinstance "Intensity" 0.0 :!class /Script/Engine.MaterialInstanceDynamic)))

(event EventBeginPlay
  (bind _returnvalue (Transformation|GetActorTransform))
  (if (Variables|Default|GetIsTraversible)
    (Utilities|FlowControl|Sequence
      (:then_0
        (bind _outhit (Collision|LineTraceByChannel (.location _returnvalue) (+ (.location _returnvalue) "120.000000,0,0") "TraceTypeQuery1" false 0 "ForOneFrame"))
        (if (.bBlockingHit (Collision|BreakHitResult _outhit))
          (bind _asbp_map_tile (Utilities|Casting|CastToBP_MapTile (.HitActor (Collision|BreakHitResult _outhit))))
          (if (Variables|BP_MapTile_C|GetIsTraversible _asbp_map_tile)
            (Variables|Default|SetForwardTile _asbp_map_tile))))
      (:then_1
        (bind _outhit_2 (Collision|LineTraceByChannel (.location _returnvalue) (+ (.location _returnvalue) "-120.000000,0,0") "TraceTypeQuery1" false 0 "ForOneFrame"))
        (if (.bBlockingHit (Collision|BreakHitResult _outhit_2))
          (bind _asbp_map_tile_2 (Utilities|Casting|CastToBP_MapTile (.HitActor (Collision|BreakHitResult _outhit_2))))
          (if (Variables|BP_MapTile_C|GetIsTraversible _asbp_map_tile_2)
            (Variables|Default|SetBackTile _asbp_map_tile_2))))
      (:then_2
        (bind _outhit_3 (Collision|LineTraceByChannel (.location _returnvalue) (+ (.location _returnvalue) "0.000000,120.000000,0") "TraceTypeQuery1" false 0 "None"))
        (if (.bBlockingHit (Collision|BreakHitResult _outhit_3))
          (bind _asbp_map_tile_3 (Utilities|Casting|CastToBP_MapTile (.HitActor (Collision|BreakHitResult _outhit_3))))
          (if (Variables|BP_MapTile_C|GetIsTraversible _asbp_map_tile_3)
            (Variables|Default|SetRightTile _asbp_map_tile_3))))
      (:then_3
        (bind _outhit_4 (Collision|LineTraceByChannel (.location _returnvalue) (+ (.location _returnvalue) "0.000000,-120.000000,0") "TraceTypeQuery1" false 0 "ForOneFrame"))
        (if (.bBlockingHit (Collision|BreakHitResult _outhit_4))
          (bind _asbp_map_tile_4 (Utilities|Casting|CastToBP_MapTile (.HitActor (Collision|BreakHitResult _outhit_4))))
          (if (Variables|BP_MapTile_C|GetIsTraversible _asbp_map_tile_4)
            (Variables|Default|SetLeftTile _asbp_map_tile_4)))))))

(fn ConstructionScript
  (bind _returnvalue (Rendering|Material|CreateDynamicMaterialInstance (Variables|Default|GetTileMesh) 0 "/Game/Materials/TileMaterial_Inst.TileMaterial_Inst" "None" :!class /Script/Engine.PrimitiveComponent))
  (Variables|Default|SetMaterialInstance _returnvalue)
  (Rendering|Material|SetVectorParameterValue (Variables|Default|GetMaterialInstance) "BorderColor" (Variables|Default|GetDefaultColor) :!class /Script/Engine.MaterialInstanceDynamic)
  (Rendering|Material|SetScalarParameterValue (Variables|Default|GetMaterialInstance) "Intensity" (Variables|Default|GetDefaultIntensity) :!class /Script/Engine.MaterialInstanceDynamic))

(fn GetConnectedTiles
  (return (Utilities|Array|MakeArray (Variables|Default|GetForwardTile) (Variables|Default|GetBackTile) (Variables|Default|GetRightTile) (Variables|Default|GetLeftTile))))