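; BP_GameState tracks turn count and action points for a turn-based game.
; A turn change fires a dispatcher, increments the turn, then plays a timeline that broadcasts its time each update and signals when finished.
; Spending action points reduces the pool and, once it is empty, tells BP_Gamemode that the player died.
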(event Custom|Use%20Action%20Points
  (params (Amount :type Integer))
  (bind _output_get (Variables|Default|SetAction%20Points (- (Variables|Default|GetAction%20Points) Amount)))
  (if (<= _output_get 0)
    (bind _asbp_gamemode (Utilities|Casting|CastToBP_Gamemode (Game|GetGameMode)))
    (Default|YouDied _asbp_gamemode true)))

(event Custom|Turn%20Change_Event
  (Default|CallTurnChange)
  (Math|Integer|IncrementInt (Variables|Default|GetTurn)
    (:%20%20
      (bind _time (Timeline|TurnAnimation PlayFromStart)
        (:Update
          (Default|CallTurnAnimationTick _time))
        (:Finished
          (Default|CallTurnAnimationFinished))))))

(fn ConstructionScript)