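; BP_NPC is a turn-based NPC that advances one tile along its PathTiles route each turn.
; BeginPlay binds MoveToNextTile to BP_GameState's turn change and optionally starts the route backward.
; Tick interpolates the actor to a point above the next tile, then either reverses or wraps around at path ends, depending on BackAndForth.
; A death event plays a randomly pitched sound and destroys the actor.
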(event Custom|MoveToNextTile
  (if (> (Utilities|Array|Length (Variables|Default|GetPathTiles)) 1)
    (Variables|Default|SetIsMoving true)))

(event Custom|Fucking%20die
  ;[1 1 1] Death
  (Audio|PlaySoundatLocation "/Game/Sounds/ow.ow" (Transformation|GetActorLocation) "0, 0, 0" 1.0 (Math|Random|RandomFloatinRange 0.8 1.2) 0.0 0 0 0 0)
  (Actor|DestroyActor))

(event EventBeginPlay
  (if (Variables|Default|GetStartBackward)
    (Variables|Default|SetIsReversing true)
    (Variables|Default|SetCurrentPosition (Utilities|Array|Length (Variables|Default|GetPathTiles))))
  (bind _asbp_game_state (Utilities|Casting|CastToBP_GameState (Game|GetGameState)))
  (EventDispatchers|BindEventtoTurnChange _asbp_game_state (delegate Custom|MoveToNextTile)))

(event Collision|EventActorBeginOverlap
  (params (OtherActor :type Actor%20Object%20Reference)))

(event EventTick
  (params (DeltaSeconds :type Float%20%28single-precision%29))
  ;[1 1 1] Movement
  (if (Variables|Default|GetIsMoving)
    (if (Variables|Default|GetIsReversing)
      ;;[1 1 1] Backward
      (Transformation|SetActorLocation (Math|Interpolation|VInterpTo (Transformation|GetActorLocation) (+ (Transformation|GetActorLocation (Utilities|Array|Get(acopy) (Variables|Default|GetPathTiles) (+ (Variables|Default|GetCurrentPosition) -1))) "0,0,30.000000") DeltaSeconds (Variables|Default|GetMoveSpeed)) false false)
      (if (Utilities|Operators|EqualEqual (Transformation|GetActorLocation) (+ (Transformation|GetActorLocation (Utilities|Array|Get(acopy) (Variables|Default|GetPathTiles) (+ (Variables|Default|GetCurrentPosition) -1))) "0,0,30.000000") 0.5)
        (Variables|Default|SetIsMoving false)
        (bind _output_get (Variables|Default|SetCurrentPosition (+ (Variables|Default|GetCurrentPosition) -1)))
        (if (<= _output_get 0)
          (if (Variables|Default|GetBackAndForth)
            (Variables|Default|SetIsReversing false)
            (else
              (Variables|Default|SetCurrentPosition (Utilities|Array|Length (Variables|Default|GetPathTiles)))))))
      (else
        ;;[1 1 1] Forward
        (Transformation|SetActorLocation (Math|Interpolation|VInterpTo (Transformation|GetActorLocation) (+ (Transformation|GetActorLocation (Utilities|Array|Get(acopy) (Variables|Default|GetPathTiles) (+ (Variables|Default|GetCurrentPosition) 1))) "0,0,30.000000") DeltaSeconds (Variables|Default|GetMoveSpeed)) false false)
        (if (Utilities|Operators|EqualEqual (Transformation|GetActorLocation) (+ (Transformation|GetActorLocation (Utilities|Array|Get(acopy) (Variables|Default|GetPathTiles) (+ (Variables|Default|GetCurrentPosition) 1))) "0,0,30.000000") 0.5)
          (Variables|Default|SetIsMoving false)
          (bind _output_get_2 (Variables|Default|SetCurrentPosition (+ (Variables|Default|GetCurrentPosition) 1)))
          (if (>= _output_get_2 (Utilities|Array|LastIndex (Variables|Default|GetPathTiles)))
            (if (Variables|Default|GetBackAndForth)
              (Variables|Default|SetIsReversing true)
              (else
                (Variables|Default|SetCurrentPosition -1)))))))))

(fn ConstructionScript)